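; Court floor actor for a duel mode that drives a dynamic material on its plane to reflect the state of the match.
; Each tick it reads the court percentage from DueloGameState and enables radial mode whenever the split is not even.
; In that mode, any player below the vital-points threshold sets the circle's center to their pawn, with radius proportional to remaining points.
; The circle inverts according to which side of the floor's Y position that pawn occupies.
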(event `self.ReceiveBeginPlay`
  (bind _returnvalue (`PrimitiveComponent.CreateDynamicMaterialInstance` (`self.Plane`) 0 null "None"))
  (set `self.MatDinamico` _returnvalue))

(event `self.ReceiveTick`
  (params (DeltaSeconds :type "Float (single-precision)"))
  (bind _matdinamico (`self.MatDinamico`))
  (bind _asduelo_game_state (cast `DueloGameState` (`GameplayStatics.GetGameState`)))
  (if (== (`DueloGameState.PorcentajeCanchaA` _asduelo_game_state) 0.5)
    (`MaterialInstanceDynamic.SetScalarParameterValue` _matdinamico "ModoRadial" 0.0)
    (else
      (`MaterialInstanceDynamic.SetScalarParameterValue` _matdinamico "ModoRadial" 1.0)
      (for _array_element (`GameStateBase.PlayerArray` (`GameplayStatics.GetGameState`))
        (bind _returnvalue (`PlayerState.GetPawn` _array_element))
        (`/Engine/EditorBlueprintResources/StandardMacros.IsValid` _returnvalue
          (:`Is Valid`
            (bind _asduelo_player_state (cast `DueloPlayerState` _array_element))
            (bind _puntosvitales (`DueloPlayerState.PuntosVitales` _asduelo_player_state))
            (if (< _puntosvitales 1250)
              (bind _returnvalue_2 (`self.K2_GetActorLocation` _returnvalue))
              (`MaterialInstanceDynamic.SetVectorParameterValue` _matdinamico "PosicionPerdedor" (`KismetMathLibrary.Conv_VectorToLinearColor` _returnvalue_2))
              (`MaterialInstanceDynamic.SetScalarParameterValue` _matdinamico "InvertirCirculo" (`KismetMathLibrary.SelectFloat` 1.0 0.0 (< (.y _returnvalue_2) (.y (`self.K2_GetActorLocation`)))))
              (`MaterialInstanceDynamic.SetScalarParameterValue` _matdinamico "RadioCirculo" (* (/ (`KismetMathLibrary.Conv_IntToDouble` _puntosvitales) 1250.0) 600.0)))))))))

(fn `UserConstructionScript`)